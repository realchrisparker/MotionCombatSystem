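; Sword attack chooser for the player's motion combat system, which scores attack entries for selection.
; ScoreAttack currently passes straight through to the built-in C++ parent scoring.
; An unconnected example path shows custom scoring: selection weight plus tag, distance, direction and situation helper scores, combined by AggregateScore.
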(fn `ScoreAttack`
  (params (Entry :type "MCS_AttackEntry Structure (by ref)") (Instigator :type "Actor Object Reference") (Targets :type "Array of Actor Object Reference (by ref)") (DesiredDirection :type "EMCS_AttackDirection Enum" :default "Forward") (CurrentSituation :type "MCS_AttackSituation Structure (by ref)"))
  (returns (ReturnValue :type "Float (single-precision)"))
  (locals (CustomBaseScore :type "Float (double-precision)") (CustomTagScore :type "Float (double-precision)") (CustomDistanceScore :type "Float (double-precision)") (CustomDirectionScore :type "Float (double-precision)") (CustomSituationScore :type "Float (double-precision)"))
  (return (`parent.ScoreAttack` Entry Instigator Targets DesiredDirection CurrentSituation)))