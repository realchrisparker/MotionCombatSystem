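; Player character Blueprint that uses Motion Combat System (MCS) components for melee attacks and hit damage.
; On BeginPlay it activates the unarmed attack set through the core component, and on possession it caches the BP_PlayerController.
; Hitbox hits on Characters apply the attack entry's damage as point damage and print the result on screen.
; Getter functions expose both MCS components and the mesh's AnimInstance.
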(event `self.ReceiveBeginPlay`
  ;[1 1 1] Start with unarmed attack set
  (`self.SetActiveAttackSetByTag` (struct :`TagName` "MCS.Attacks.Unarmed")))

(event `self.ReceivePossessed`
  (params (NewController :type "Controller Object Reference"))
  (if (`Controller.IsPlayerController` NewController)
    (bind _asbp_player_controller (cast `/Game/Player/BP_PlayerController` NewController))
    (set `self.MyPlayerController` _asbp_player_controller)))

(event `self.Motion Combat System Core Component.OnTargetingUpdated`
  (params (NewTargetList :type "Array of MCS_TargetInfo Structure (by ref)") (NumTargets :type Integer)))

(event `self.Motion Combat System Hitbox Component.OnHitboxHit`
  (params (HitActor :type "Actor Object Reference") (HitResult :type "HitResult Structure (by ref)") (AttackEntry :type "MCS_AttackEntry Structure"))
  (bind _returnvalue (`GameplayStatics.GetPlayerController` 0))
  ;[1 1 1] Send damage to hit actor
  (`KismetSystemLibrary.IsObjectOfSoftClass` HitActor "/Script/Engine.Character"
    (:`True`
      (bind _returnvalue_2 (`GameplayStatics.ApplyPointDamage` HitActor (`.Damage` (break `MCS_AttackEntry` AttackEntry)) (`.ImpactPoint` (`GameplayStatics.BreakHitResult` HitResult)) HitResult _returnvalue (`self.GetOwner` _returnvalue)))
      (`KismetSystemLibrary.PrintText` (`|FormatText` "Damage: {d}" _returnvalue_2) true false (struct :`A` 1.0) 5.0))))

(fn `GetCharacterAnimInstance`
  (returns (AnimInstance :type "AnimInstance Object Reference"))
  (bind _mesh (`self.Mesh`)
    (:`then`
      (return (`SkeletalMeshComponent.GetAnimInstance` _mesh)))
    (:`else`
      (return null))))

(fn `GetMCSCoreComponent`
  (returns (NewParam :type "MCS_CombatCoreComponent Object Reference"))
  (bind _motion_combat_system_core_component (`self.Motion Combat System Core Component`)
    (:`then`
      (return _motion_combat_system_core_component))
    (:`else`
      (return null))))

(fn `GetMCSHitboxComponent`
  (returns (NewParam :type "MCS_CombatHitboxComponent Object Reference"))
  (bind _motion_combat_system_hitbox_component (`self.Motion Combat System Hitbox Component`)
    (:`then`
      (return _motion_combat_system_hitbox_component))
    (:`else`
      (return null))))

(fn `SetActiveAttackSetByTag`
  (params (Tag :type "GameplayTag Structure"))
  (returns (Success :type Boolean))
  (bind _returnvalue (`MCS_CombatCoreComponent.SetActiveAttackSet` (`self.Motion Combat System Core Component`) Tag))
  (return _returnvalue))

(fn `UserConstructionScript`)